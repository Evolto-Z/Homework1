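; Game state Blueprint that holds round data: time left, a round-over flag, and the winner's name and score.
; On BeginPlay it runs ResetGameState, which copies MaxTimeLeft into TimeLeft, then zeroes MaxTimeLeft and clears the round and winner fields.
; RoundOver's RepNotify calls RoundOverEvent on MyGameInstance to pass on the round end.
; RepNotifies for GameStartTimer and RandomTimerValue1 are empty.
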(event `self.ReceiveBeginPlay`
  (`self.Reset Game State`))

(fn `OnRep_GameStartTimer`)

(fn `OnRep_RandomTimerValue1`)

(fn `OnRep_RoundOver`
  (bind _asmy_game_instance (cast `/Game/Blueprints/MyGameInstance` (`GameplayStatics.GetGameInstance`)))
  (`/Game/Blueprints/MyGameInstance.RoundOverEvent` _asmy_game_instance))

(fn `Reset Game State`
  (set `self.TimeLeft` (`self.MaxTimeLeft`))
  (set `self.RoundOver` false)
  (set `self.MaxTimeLeft` 0.0)
  (set `self.WinnerName` "")
  (set `self.WinnerScore` 0))

(fn `UserConstructionScript`)