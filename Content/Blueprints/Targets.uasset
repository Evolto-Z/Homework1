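; Targets is a shootable target actor that moves in a circle and awards score when hit by a projectile.
; Each tick the server advances an angle, positions the sphere on the X-Z plane and stores its world location in CurLocation.
; Remote clients apply that location through an OnRep function.
; On a BP_Projectile hit, the server increments the instigator's MyPlayerState score, then destroys target and projectile.
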(event `self.ReceiveTick`
  (params (DeltaSeconds :type "Float (single-precision)"))
  (`self.MoveAround` DeltaSeconds))

(event `MoveAround`
  (params (DeltaTime :type "Float (double-precision)"))
  (bind _sphere (`self.Sphere`))
  (bind _radius (`self.radius`))
  (bind _theta (`self.theta`))
  (bind _returnvalue (+ (* DeltaTime (`self.angularVel`)) (`self.theta`)))
  (`/Engine/EditorBlueprintResources/ActorMacros.Switch Has Authority`
    (:`Authority`
      (if (>= _returnvalue 360.0)
        (set `self.theta` (- _returnvalue 360.0))
        (else
          (set `self.theta` _returnvalue)))
      (`SceneComponent.K2_SetRelativeLocation` _sphere (`KismetMathLibrary.MakeVector` (* _radius (`KismetMathLibrary.DegCos` _theta)) 0.0 (* _radius (`KismetMathLibrary.DegSin` _theta))) false false)
      (set `self.curLocation` (`SceneComponent.K2_GetComponentLocation` _sphere)))))

(event `self.Sphere.OnComponentHit`
  (params (HitComponent :type "PrimitiveComponent Object Reference") (OtherActor :type "Actor Object Reference") (OtherComp :type "PrimitiveComponent Object Reference") (NormalImpulse :type "Vector Structure") (Hit :type "HitResult Structure (by ref)"))
  (`/Engine/EditorBlueprintResources/ActorMacros.Switch Has Authority`
    (:`Authority`
      (bind _asbp_projectile (cast `/Game/Blueprints/BP_Projectile` OtherActor))
      (bind _asmy_player_state (cast `/Game/Blueprints/MyPlayerState` (`Controller.PlayerState` (`self.GetInstigatorController` _asbp_projectile))))
      (`/Game/Blueprints/MyPlayerState.IncrementScore` _asmy_player_state)
      (`self.K2_DestroyActor`)
      (`self.K2_DestroyActor` _asbp_projectile))))

(fn `OnRep_curLocation`
  (`/Engine/EditorBlueprintResources/ActorMacros.Switch Has Authority`
    (:`Remote`
      (`SceneComponent.K2_SetWorldLocation` (`self.Sphere`) (`self.curLocation`) false false))))

(fn `UserConstructionScript`)